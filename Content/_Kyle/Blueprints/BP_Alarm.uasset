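; BP_Alarm is an alarm actor that, when triggered, alerts enemies and starts reinforcement spawning.
; ServerTurnOnAlarm calls ClientTurnOnAlarm, which swaps the cylinder's material, shows a HUD warning for player 0 and plays an attached alarm sound.
; The same client-named event then messages every BPI_Enemy actor and calls ServerStartSpawning on the BP_Enemy_Spawner found in the level.
; Both alerting and spawning are skipped if the player character cast fails.
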(event `Server Turn On Alarm`
  (`self.Client Turn On Alarm`))

(event `Client Turn On Alarm`
  (`PrimitiveComponent.SetMaterial` (`self.Cylinder`) 0 "/Game/_Kyle/Materials/MAT_Alarm_On.MAT_Alarm_On")
  (bind _asbp_third_person_character (cast `/Game/ThirdPerson/Blueprints/BP_ThirdPersonCharacter` (`GameplayStatics.GetPlayerCharacter` 0)))
  (`/Game/_Kyle/UI/WB_HUD.Show HUD Message` (`/Game/ThirdPerson/Blueprints/BP_ThirdPersonCharacter.HUD` _asbp_third_person_character) "Alarms Raised! reinforcements incoming!")
  (`GameplayStatics.SpawnSoundAttached` "/Game/_Kyle/Audio/SC_Alarm.SC_Alarm" (`self.Cylinder`) "None" (0.0 0.0 0.0) (struct) "KeepRelativeOffset" false 1.0 1.0 0.0 null null)
  (bind _outactors (`GameplayStatics.GetAllActorsWithInterface` "/Game/_Kyle/Blueprints/AI/BPI_Enemy.BPI_Enemy_C"))
  (for _array_element _outactors
    (message `/Game/_Kyle/Blueprints/AI/BPI_Enemy.Alarms Raised` _array_element))
  (bind _returnvalue (`GameplayStatics.GetActorOfClass` "/Game/_Kyle/Blueprints/BP_Enemy_Spawner.BP_Enemy_Spawner_C"))
  (`/Game/_Kyle/Blueprints/BP_Enemy_Spawner.Server Start Spawning` _returnvalue))

(fn `UserConstructionScript`)