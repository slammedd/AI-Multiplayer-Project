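; Behavior tree task that makes an explosive robot chase its blackboard TargetActor and explode on reaching it.
; If the robot is not already chasing, it first switches to chase speed and has player 0's character raise all alarms through ServerRaiseAllAlarms.
; AI MoveTo then runs, calling ServerExplode and finishing successfully on arrival, or failing the task if the move fails.
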(event `self.ReceiveExecuteAI`
  (params (OwnerController :type "AIController Object Reference") (ControlledPawn :type "Pawn Object Reference"))
  (bind _asbp_explosive_robot (cast `/Game/_Kyle/Blueprints/AI/BP_Explosive_Robot` ControlledPawn))
  (if (not (`/Game/_Kyle/Blueprints/AI/BP_Explosive_Robot.Chasing` _asbp_explosive_robot))
    (`/Game/_Kyle/Blueprints/AI/BP_Explosive_Robot.Chase Speed` _asbp_explosive_robot)
    (bind _asbp_third_person_character (cast `/Game/ThirdPerson/Blueprints/BP_ThirdPersonCharacter` (`GameplayStatics.GetPlayerCharacter` 0)))
    (`/Game/ThirdPerson/Blueprints/BP_ThirdPersonCharacter.Server Raise All Alarms` _asbp_third_person_character))
  (`|AIMoveTo` _asbp_explosive_robot (0.0 0.0 0.0) (`BTFunctionLibrary.GetBlackboardValueAsActor` (`self.Target Actor`)) 50.0 true
    (:`OnSuccess`
      (`/Game/_Kyle/Blueprints/AI/BP_Explosive_Robot.Server Explode` _asbp_explosive_robot)
      (`self.FinishExecute` true))
    (:`OnFail`
      (`self.FinishExecute` false))))