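; Explosive robot AI enemy that spins its sphere as it moves, faster when chasing, and can explode to hurt the player.
; Sight perception and alarm events set the Blackboard target, while speed events toggle chase state and alarm material.
; Exploding enlarges an overlap sphere for one-time authority-side damage, then the player character destroys the robot.
; Server-to-Client event pairs relay explosions, alarms and damage, with death by damage spawning a random drop.
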(event `self.ReceiveTick`
  (params (DeltaSeconds :type "Float (single-precision)"))
  (if (> (`KismetMathLibrary.VSize` (`self.GetVelocity`)) 0.0)
    (if (`self.Chasing`)
      (`SceneComponent.K2_AddLocalRotation` (`self.Sphere`) (struct :`Pitch` 5.0) false false)
      (else
        (`SceneComponent.K2_AddLocalRotation` (`self.Sphere`) (struct :`Pitch` 1.0) false false)))))

(event `Server Explode`
  (`self.Client Explode`))

(event `Client Explode`
  (`GameplayStatics.SpawnEmitterAtLocation` "/Game/StarterContent/Particles/P_Explosion.P_Explosion" (`self.K2_GetActorLocation`) (struct) (5.0 5.0 5.0))
  (`GameplayStatics.PlaySoundAtLocation` "/Game/StarterContent/Audio/Explosion_Cue.Explosion_Cue" (`self.K2_GetActorLocation`) (struct) 1.0 1.0 0.0 null null null null)
  (`SphereComponent.SetSphereRadius` (`self.Sphere2`) 500.0 true)
  (`KismetSystemLibrary.Delay` 0.2)
  (bind _asbp_third_person_character (cast `/Game/ThirdPerson/Blueprints/BP_ThirdPersonCharacter` (`GameplayStatics.GetPlayerCharacter` 0)))
  (`/Game/ThirdPerson/Blueprints/BP_ThirdPersonCharacter.Server Destroy Actor` _asbp_third_person_character self))

(event `Server Change Material`
  (`self.Client Change Material`))

(event `Chase Speed`
  ;[1 1 1] Speed Control
  (set `self.Chasing` true)
  (set `CharacterMovementComponent.MaxWalkSpeed` 400.0 (`self.CharacterMovement`))
  (`self.Server Change Material`))

(event `Client Change Material`
  (`PrimitiveComponent.SetMaterial` (`self.Sphere1`) 0 "/Game/_Kyle/Materials/MAT_Alarm_On.MAT_Alarm_On"))

(event `Walk Speed`
  ;[1 1 1] Speed Control
  (set `self.Chasing` false)
  (set `CharacterMovementComponent.MaxWalkSpeed` 150.0 (`self.CharacterMovement`)))

(event `self.ReceiveBeginPlay`
  (set `self.Blackboard` (`AIBlueprintHelperLibrary.GetBlackboard` null)))

(event `self.Sphere2.OnComponentBeginOverlap`
  (params (OverlappedComponent :type "PrimitiveComponent Object Reference") (OtherActor :type "Actor Object Reference") (OtherComp :type "PrimitiveComponent Object Reference") (OtherBodyIndex :type Integer) (bFromSweep :type Boolean) (SweepResult :type "HitResult Structure (by ref)"))
  (`/Engine/EditorBlueprintResources/ActorMacros.Switch Has Authority`
    (:`Authority`
      (bind _asbp_third_person_character (cast `/Game/ThirdPerson/Blueprints/BP_ThirdPersonCharacter` OtherActor))
      (`/Engine/EditorBlueprintResources/StandardMacros.DoOnce` false
        (:`Completed`
          (`/Game/ThirdPerson/Blueprints/BP_ThirdPersonCharacter.Server Damage Player` _asbp_third_person_character 25.0))))))

(event `self.AIPerception.OnTargetPerceptionUpdated`
  (params (Actor :type "Actor Object Reference") (Stimulus :type "AIStimulus Structure"))
  (`self.Sight` Actor Stimulus))

(event `self.Damage Enemy`
  (params (Damage :type "Float (double-precision)"))
  (`self.Server Damage Enemy` Damage))

(event `Server Damage Enemy`
  (params (Damage :type "Float (double-precision)"))
  (`self.Client Damage Enemy` Damage))

(event `Client Damage Enemy`
  (params (Damage :type "Float (double-precision)"))
  (bind _returnvalue (`self.K2_GetActorLocation`))
  (bind _blackboard (`self.Blackboard`))
  (bind _output_get (set `self.Health` (- (`self.Health`) Damage)))
  (if (<= _output_get 0.0)
    (`/Engine/EditorBlueprintResources/StandardMacros.DoOnce` false
      (:`Completed`
        (`MovementComponent.StopMovementImmediately` (`self.CharacterMovement`))
        (set `self.Dead` true)
        (`/Engine/EditorBlueprintResources/StandardMacros.IsValid` _blackboard
          (:`Is Valid`
            (`BlackboardComponent.SetValueAsBool` _blackboard "Enemy Dead" true)
            (set `self.Can Shoot` false)
            (`GameplayStatics.PlaySoundAtLocation` "/Game/StarterContent/Audio/Explosion_Cue.Explosion_Cue" _returnvalue (struct) 1.0 1.0 0.0 null null null null)
            (`GameplayStatics.SpawnEmitterAtLocation` "/Game/StarterContent/Particles/P_Explosion.P_Explosion" _returnvalue (struct) (5.0 5.0 5.0))
            (`AIController.K2_ClearFocus` (`AIBlueprintHelperLibrary.GetAIController` self))
            (`|SpawnActorFromClass` (`KismetArrayLibrary.Array_Random` (`self.Drops`)) (`self.GetTransform`) "Undefined" "MultiplyWithRoot" null null)
            (`self.K2_DestroyActor`)))))
    (else
      (`self.PlayAnimMontage` "/Game/_Kyle/Animations/AM_Hit_React.AM_Hit_React")
      (`GameplayStatics.PlaySoundAtLocation` "/Game/_Kyle/Audio/SC_Robot_Damage.SC_Robot_Damage" (`self.K2_GetActorLocation`) (struct) 1.0 1.0 0.0 null null null null))))

(event `self.Alarms Raised`
  (`self.Server Alarms Raised`))

(event `Server Alarms Raised`
  (`self.Client Alarms Raised`))

(event `Client Alarms Raised`
  (`BlackboardComponent.SetValueAsBool` (`self.Blackboard`) "Alarms Raised" true)
  (`BlackboardComponent.SetValueAsObject` (`self.Blackboard`) "Target Actor" (`GameplayStatics.GetPlayerCharacter` 0)))

(fn `Sight`
  (params (Actor :type "Actor Object Reference") (Stimulus :type "AIStimulus Structure"))
  (bind _asbp_third_person_character (cast `/Game/ThirdPerson/Blueprints/BP_ThirdPersonCharacter` Actor)
    (:`then`
      (`BlackboardComponent.SetValueAsObject` (`self.Blackboard`) "Target Actor" _asbp_third_person_character)
      (set `self.Target Actor` _asbp_third_person_character)
      (set `self.Focal Actor` _asbp_third_person_character))
    (:`CastFailed`
      (return))))

(fn `UserConstructionScript`)