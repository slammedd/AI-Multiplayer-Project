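; Behavior tree task that walks an AI pawn around a looping patrol route taken from its AIBehaviour component.
; The PatrolPath map's keys are waypoint actors and its values are wait times, floored at 0.1 seconds.
; Move and wait steps chain through paired Server/Client events, advancing and wrapping the index.
; It finishes only on failure (missing component, empty path or failed move), otherwise patrolling indefinitely.
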(event `self.ReceiveExecuteAI`
  (params (OwnerController :type "AIController Object Reference") (ControlledPawn :type "Pawn Object Reference"))
  (bind _returnvalue (`Actor.GetComponentByClass` ControlledPawn "/Game/_Kyle/Blueprints/AI/AIBehaviour.AIBehaviour_C"))
  (bind _patrol_path (`/Game/_Kyle/Blueprints/AI/AIBehaviour.Patrol Path` _returnvalue))
  (`/Engine/EditorBlueprintResources/StandardMacros.IsValid` _returnvalue
    (:`Is Valid`
      (if (> (`BlueprintMapLibrary.Map_Length` _patrol_path) 0)
        (set `self.Patrol Path` _patrol_path)
        (`self.Server Move to Patrol Point`)
        (else
          (`self.FinishExecute` false))))
    (:`Is Not Valid`
      (`self.FinishExecute` false))))

(event `Server Move to Patrol Point`
  (`self.Client Move to Patrol Point`))

(event `Client Move to Patrol Point`
  (bind _patrol_path (`self.Patrol Path`))
  (bind _keys (`BlueprintMapLibrary.Map_Keys` (`self.Patrol Path`)))
  (`|AIMoveTo` (stale `self.ReceiveExecuteAI` ControlledPawn) (`Actor.K2_GetActorLocation` (`|GetArrayItem` _keys (`self.Current Patrol Index`))) null
    (:`OnSuccess`
      (bind _keys_2 (`BlueprintMapLibrary.Map_Keys` _patrol_path))
      (`KismetSystemLibrary.Delay` (`KismetMathLibrary.FMax` (`BlueprintMapLibrary.Map_Find` _patrol_path (`|GetArrayItem` _keys_2 (`self.Current Patrol Index`))) 0.1))
      (`self.Server On End Waiting`))
    (:`OnFail`
      (`self.FinishExecute` false))))

(event `Client On End Waiting`
  (bind _result (`/Engine/EditorBlueprintResources/StandardMacros.IncrementInt` (`self.Current Patrol Index`))
    (:`  `
      (if (>= _result (`BlueprintMapLibrary.Map_Length` (`self.Patrol Path`)))
        (set `self.Current Patrol Index` 0)
        (`self.Server Move to Patrol Point`)
        (else
          (`self.Server Move to Patrol Point`))))))

(event `Server On End Waiting`
  (`self.Client On End Waiting`))