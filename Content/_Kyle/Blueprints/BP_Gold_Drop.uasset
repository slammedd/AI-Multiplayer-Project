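; BP_Gold_Drop is a gold pickup that adds one Gold to the player state of the BP_ThirdPersonCharacter overlapping its Box.
; If that character's HUD is valid, it shows a collection message, plays the pickup sound and asks the character's ServerDestroyActor to remove the drop.
; Sound and destruction depend on the HUD check, while the Gold increment happens before it.
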(event `self.Box.OnComponentBeginOverlap`
  (params (OverlappedComponent :type "PrimitiveComponent Object Reference") (OtherActor :type "Actor Object Reference") (OtherComp :type "PrimitiveComponent Object Reference") (OtherBodyIndex :type Integer) (bFromSweep :type Boolean) (SweepResult :type "HitResult Structure (by ref)"))
  (bind _asbp_third_person_character (cast `/Game/ThirdPerson/Blueprints/BP_ThirdPersonCharacter` OtherActor))
  (bind _asbp_player_state (cast `/Game/_Kyle/Blueprints/BP_Player_State` (`Pawn.PlayerState` _asbp_third_person_character)))
  (`/Engine/EditorBlueprintResources/StandardMacros.IncrementInt` (`/Game/_Kyle/Blueprints/BP_Player_State.Gold` _asbp_player_state)
    (:`  `
      (bind _hud (`/Game/ThirdPerson/Blueprints/BP_ThirdPersonCharacter.HUD` _asbp_third_person_character))
      (`/Engine/EditorBlueprintResources/StandardMacros.IsValid` _hud
        (:`Is Valid`
          (`/Game/_Kyle/UI/WB_HUD.Show HUD Message` _hud "Gold Collected!")
          (`GameplayStatics.PlaySoundAtLocation` "/Game/_Kyle/Audio/SC_Pickup.SC_Pickup" (`self.K2_GetActorLocation`) (struct) 1.0 1.0 0.0 null null null null)
          (`/Game/ThirdPerson/Blueprints/BP_ThirdPersonCharacter.Server Destroy Actor` _asbp_third_person_character self))))))

(fn `UserConstructionScript`)