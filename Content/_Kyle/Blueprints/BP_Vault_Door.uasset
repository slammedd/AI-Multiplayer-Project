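; BP_Vault_Door is a vault door that opens once, when a third-person character overlaps its Box.
; The overlap calls ServerOpenVault, which forwards to ClientOpenVault, where a DoOnce gate plays the door sound.
; It then shows a drilling-finished HUD message to player 0's character and runs the Opening timeline, which drives the yaw of the Arrow component.
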(event `Server Open Vault`
  (`self.Client Open Vault`))

(event `Client Open Vault`
  (`/Engine/EditorBlueprintResources/StandardMacros.DoOnce` false
    (:`Completed`
      (`GameplayStatics.PlaySoundAtLocation` "/Game/_Kyle/Audio/SC_Vault_Door.SC_Vault_Door" (`self.K2_GetActorLocation`) (struct) 1.0 1.0 0.0 null null null null)
      (bind _asbp_third_person_character (cast `/Game/ThirdPerson/Blueprints/BP_ThirdPersonCharacter` (`GameplayStatics.GetPlayerCharacter` 0)))
      (`/Game/_Kyle/UI/WB_HUD.Show HUD Message` (`/Game/ThirdPerson/Blueprints/BP_ThirdPersonCharacter.HUD` _asbp_third_person_character) "Drilling Process Finished! Vault Opening!")
      (bind (_direction _z_roation) (`Timeline|Opening`)
        (:`Update`
          (`SceneComponent.K2_SetRelativeRotation` (`self.Arrow`) (`KismetMathLibrary.MakeRotator` 0.0 0.0 _z_roation) false false))))))

(event `self.Box.OnComponentBeginOverlap`
  (params (OverlappedComponent :type "PrimitiveComponent Object Reference") (OtherActor :type "Actor Object Reference") (OtherComp :type "PrimitiveComponent Object Reference") (OtherBodyIndex :type Integer) (bFromSweep :type Boolean) (SweepResult :type "HitResult Structure (by ref)"))
  (cast `/Game/ThirdPerson/Blueprints/BP_ThirdPersonCharacter` OtherActor)
  (`self.Server Open Vault`))

(fn `UserConstructionScript`)