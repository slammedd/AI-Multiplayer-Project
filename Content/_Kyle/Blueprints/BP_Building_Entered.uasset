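; BP_Building_Entered is a trigger actor that advances the objective when a third-person character enters its box.
; The first overlap calls its Server-to-Client objective event chain, which sets CurrentObjective on player character 0 to a fixed enum value.
; It then calls the overlapping character's ServerChangeObjective and has that character destroy the trigger through ServerDestroyActor.
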(event `self.Box.OnComponentBeginOverlap`
  (params (OverlappedComponent :type "PrimitiveComponent Object Reference") (OtherActor :type "Actor Object Reference") (OtherComp :type "PrimitiveComponent Object Reference") (OtherBodyIndex :type Integer) (bFromSweep :type Boolean) (SweepResult :type "HitResult Structure (by ref)"))
  (bind _asbp_third_person_character (cast `/Game/ThirdPerson/Blueprints/BP_ThirdPersonCharacter` OtherActor))
  (`/Engine/EditorBlueprintResources/StandardMacros.DoOnce` false
    (:`Completed`
      (`self.Server Set Objective`)
      (`/Game/ThirdPerson/Blueprints/BP_ThirdPersonCharacter.Server Change Objective` _asbp_third_person_character)
      (`/Game/ThirdPerson/Blueprints/BP_ThirdPersonCharacter.Server Destroy Actor` _asbp_third_person_character self))))

(event `Server Set Objective`
  (`self.Client Set Objective`))

(event `Client Set Objective`
  (bind _asbp_third_person_character (cast `/Game/ThirdPerson/Blueprints/BP_ThirdPersonCharacter` (`GameplayStatics.GetPlayerCharacter` 0)))
  (set `/Game/ThirdPerson/Blueprints/BP_ThirdPersonCharacter.Current Objective` "NewEnumerator1" _asbp_third_person_character))

(fn `UserConstructionScript`)