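; BP_Spaceship is a spaceship actor that drops off and picks up via timeline-animated mesh movement along X and Z.
; Drop-off starts 20 seconds after BeginPlay, with Server events forwarding to Client events for both moves.
; Pickup turns the mesh, resets the Box trigger to unit scale and plays a second timeline in reverse.
; The first BP_ThirdPersonCharacter overlapping the Box gets ServerFinalGold called, guarded by a DoOnce.
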(event `self.ReceiveBeginPlay`
  (`KismetSystemLibrary.Delay` 20.0)
  (`self.Server Drop Off`))

(event `Server Drop Off`
  (`self.Client Drop Off`))

(event `Client Drop Off`
  (bind (_direction _z_location _x_location) (`Timeline|Drop Off`)
    (:`Update`
      (`SceneComponent.K2_SetRelativeLocation` (`self.StaticMesh`) (`KismetMathLibrary.MakeVector` _x_location 0.0 _z_location) false false))))

(event `Client Pick Up`
  (`SceneComponent.K2_SetRelativeRotation` (`self.StaticMesh`) (struct :`Yaw` 180.0) false false)
  (`SceneComponent.SetRelativeScale3D` (`self.Box`) (1.0 1.0 1.0))
  (bind (_direction _z_location _x_location) (`Timeline|Timeline` :!via `ReverseFromEnd`)
    (:`Update`
      (`SceneComponent.K2_SetRelativeLocation` (`self.StaticMesh`) (`KismetMathLibrary.MakeVector` _x_location 0.0 _z_location) false false))))

(event `Server Pick Up`
  (`self.Client Pick Up`))

(event `self.Box.OnComponentBeginOverlap`
  (params (OverlappedComponent :type "PrimitiveComponent Object Reference") (OtherActor :type "Actor Object Reference") (OtherComp :type "PrimitiveComponent Object Reference") (OtherBodyIndex :type Integer) (bFromSweep :type Boolean) (SweepResult :type "HitResult Structure (by ref)"))
  (bind _asbp_third_person_character (cast `/Game/ThirdPerson/Blueprints/BP_ThirdPersonCharacter` OtherActor))
  (`/Engine/EditorBlueprintResources/StandardMacros.DoOnce` false
    (:`Completed`
      (`/Game/ThirdPerson/Blueprints/BP_ThirdPersonCharacter.Server Final Gold` _asbp_third_person_character))))

(fn `UserConstructionScript`)