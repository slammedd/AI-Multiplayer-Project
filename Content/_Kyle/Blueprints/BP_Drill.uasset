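; BP_Drill is a vault drill that, once spawned, spins, runs a timer and opens the vault when finished.
; Timelines drive the drill's roll and the Seconds value, while a timer widget is on screen and player 0 raises all alarms after five seconds.
; On completion it removes the widget, calls the vault door, shows a HUD message and destroys itself.
; Spin, timer and destruction are routed through paired Server/Client events.
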(event `self.ReceiveBeginPlay`
  (`self.Server Spin Drill`)
  (`self.Server Drill Timer`)
  (bind _returnvalue (`|CreateWidget` "/Game/_Kyle/UI/WB_Drill_Timer.WB_Drill_Timer_C"))
  (bind _output_get (set `self.Widget` _returnvalue))
  (`UserWidget.AddToViewport` _output_get 0)
  (`KismetSystemLibrary.Delay` 5.0)
  (bind _asbp_third_person_character (cast `/Game/ThirdPerson/Blueprints/BP_ThirdPersonCharacter` (`GameplayStatics.GetPlayerCharacter` 0)))
  (`/Game/ThirdPerson/Blueprints/BP_ThirdPersonCharacter.Server Raise All Alarms` _asbp_third_person_character))

(event `Server Spin Drill`
  (`self.Client Spin Drill`))

(event `Client Spin Drill`
  (bind (_direction _x_rotation) (`Timeline|Spin`)
    (:`Update`
      (`SceneComponent.K2_SetRelativeRotation` (`self.Drill`) (`KismetMathLibrary.MakeRotator` _x_rotation) false false))))

(event `Server Destroy Actor`
  (`self.Client Destroy Actor`))

(event `Client Destroy Actor`
  (`self.K2_DestroyActor`))

(event `Server Drill Timer`
  (`self.Client Drill Timer`))

(event `Client Drill Timer`
  (bind (_direction _seconds) (`Timeline|Timer`)
    (:`Update`
      (set `self.Seconds` _seconds))
    (:`Finished`
      (`Widget.RemoveFromParent` (`self.Widget`))
      (bind _returnvalue (`GameplayStatics.GetActorOfClass` "/Game/_Kyle/Blueprints/BP_Vault_Door.BP_Vault_Door_C"))
      (`/Game/_Kyle/Blueprints/BP_Vault_Door.Server Open Vault` _returnvalue)
      (bind _asbp_third_person_character (cast `/Game/ThirdPerson/Blueprints/BP_ThirdPersonCharacter` (`GameplayStatics.GetPlayerCharacter` 0)))
      (`/Game/_Kyle/UI/WB_HUD.Show HUD Message` (`/Game/ThirdPerson/Blueprints/BP_ThirdPersonCharacter.HUD` _asbp_third_person_character) "Drilling Process Complete! Vault Opening!")
      (`self.Server Destroy Actor`))))

(fn `UserConstructionScript`)