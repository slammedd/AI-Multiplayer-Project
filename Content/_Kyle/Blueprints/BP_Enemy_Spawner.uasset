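; BP_Enemy_Spawner spawns an endless stream of enemies inside its box volume once ServerStartSpawning is called.
; Each cycle picks an explosive robot or basic guard at even odds and places it at a random point in the box.
; After a short delay, it sends the new enemy AlarmsRaisedMessage, then waits and calls the event again, with no stop condition or spawn cap.
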(event `Server Start Spawning`
  (bind _box (`self.Box`))
  (bind _box_2 (`self.Box`))
  (if (== (`KismetMathLibrary.RandomIntegerInRange` 0 1) 0)
    (bind _returnvalue (`|SpawnActorFromClass` "/Game/_Kyle/Blueprints/AI/BP_Explosive_Robot.BP_Explosive_Robot_C" (`KismetMathLibrary.MakeTransform` (`KismetMathLibrary.RandomPointInBoundingBox` (`SceneComponent.K2_GetComponentLocation` _box) (`BoxComponent.GetScaledBoxExtent` _box))) "Undefined" "MultiplyWithRoot" null null))
    (`KismetSystemLibrary.Delay` 0.2)
    (message `/Game/_Kyle/Blueprints/AI/BPI_Enemy.Alarms Raised` _returnvalue)
    (`KismetSystemLibrary.Delay` 10.0)
    (`self.Server Start Spawning`)
    (else
      (bind _returnvalue_2 (`|SpawnActorFromClass` "/Game/_Kyle/Blueprints/AI/BP_Basic_Guard.BP_Basic_Guard_C" (`KismetMathLibrary.MakeTransform` (`KismetMathLibrary.RandomPointInBoundingBox` (`SceneComponent.K2_GetComponentLocation` _box_2) (`BoxComponent.GetScaledBoxExtent` _box_2))) "Undefined" "MultiplyWithRoot" null null))
      (`KismetSystemLibrary.Delay` 0.2)
      (message `/Game/_Kyle/Blueprints/AI/BPI_Enemy.Alarms Raised` _returnvalue_2)
      (`KismetSystemLibrary.Delay` 10.0)
      (`self.Server Start Spawning`))))

(fn `UserConstructionScript`)